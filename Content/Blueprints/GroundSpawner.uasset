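; GroundSpawner is a ground tile Blueprint that extends the ground as the player moves, in the manner of an endless runner.
; On BeginPlay it caches the first BP_Character found in the level as the player.
; When the player overlaps SpawnTrigger, it spawns another GroundSpawner at its Arrow component's world transform.
; When the player overlaps DeleteTrigger, the tile destroys itself, so the chain recycles behind the player.
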(event `self.ReceiveBeginPlay`
  (bind _outactors (`GameplayStatics.GetAllActorsOfClass` "/Game/Blueprints/BP_Character.BP_Character_C"))
  (set `self.PlayerCharacter` (`|GetArrayItem` _outactors)))

(event `self.SpawnTrigger.OnComponentBeginOverlap`
  (params (OverlappedComponent :type "PrimitiveComponent Object Reference") (OtherActor :type "Actor Object Reference") (OtherComp :type "PrimitiveComponent Object Reference") (OtherBodyIndex :type Integer) (bFromSweep :type Boolean) (SweepResult :type "HitResult Structure (by ref)"))
  (if (== OtherActor (`self.PlayerCharacter`))
    (`|SpawnActorFromClass` "GroundSpawner_C" (`SceneComponent.K2_GetComponentToWorld` (`self.Arrow`)) "Undefined" "MultiplyWithRoot" null null)))

(event `self.DeleteTrigger.OnComponentBeginOverlap`
  (params (OverlappedComponent :type "PrimitiveComponent Object Reference") (OtherActor :type "Actor Object Reference") (OtherComp :type "PrimitiveComponent Object Reference") (OtherBodyIndex :type Integer) (bFromSweep :type Boolean) (SweepResult :type "HitResult Structure (by ref)"))
  (if (== OtherActor (`self.PlayerCharacter`))
    (`self.K2_DestroyActor`)))

(fn `UserConstructionScript`)