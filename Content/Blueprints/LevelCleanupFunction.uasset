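; Blueprint function LevelCleanup that clears spawned gameplay actors from the level.
; It gathers every barrel, trap, eagle, warning sign and rock with Get All Actors Of Class and destroys each one in sequential loops.
; It then destroys all ForestGroundSpawner actors except the one whose display name is "GroundSpawner", identifying the spawner to keep by a name comparison.
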(fn `Level Cleanup`
  (bind _outactors (`GameplayStatics.GetAllActorsOfClass` null "/Game/Blueprints/Obstacles/Barrel.Barrel_C"))
  (for _array_element _outactors
    (`Actor.K2_DestroyActor` _array_element))
  (bind _outactors_2 (`GameplayStatics.GetAllActorsOfClass` null "/Game/Blueprints/Obstacles/BP_Trap.BP_Trap_C"))
  (for _array_element_2 _outactors_2
    (`Actor.K2_DestroyActor` _array_element_2))
  (bind _outactors_3 (`GameplayStatics.GetAllActorsOfClass` null "/Game/Blueprints/Obstacles/BP_Eagle.BP_Eagle_C"))
  (for _array_element_3 _outactors_3
    (`Actor.K2_DestroyActor` _array_element_3))
  (bind _outactors_4 (`GameplayStatics.GetAllActorsOfClass` null "/Game/Blueprints/Obstacles/BP_WarningSign.BP_WarningSign_C"))
  (for _array_element_4 _outactors_4
    (`Actor.K2_DestroyActor` _array_element_4))
  (bind _outactors_5 (`GameplayStatics.GetAllActorsOfClass` null "/Game/Blueprints/Obstacles/BP_Rock.BP_Rock_C"))
  (for _array_element_5 _outactors_5
    (`Actor.K2_DestroyActor` _array_element_5))
  (bind _outactors_6 (`GameplayStatics.GetAllActorsOfClass` null "/Game/Blueprints/ForestGroundSpawner.ForestGroundSpawner_C"))
  (for _array_element_6 _outactors_6
    (if (`KismetStringLibrary.NotEqual_StrStr` (`KismetSystemLibrary.GetDisplayName` _array_element_6) "GroundSpawner")
      (`Actor.K2_DestroyActor` _array_element_6))))