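; Player character for an obstacle-runner level that moves itself forward each tick and tracks health, score and per-level saved high score.
; Level-begin event resets it and starts a looping timer spawning random obstacles at its Arrow, rerolling per check, so odds are uneven.
; Damage triggers timer-driven flashing, plus a physics-driven pitfall with brief intangibility for warning signs.
; Death ends the level, stops spawning and saves any new high score.
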(event `ScoreUpdater_AddScoreEvent`
  (`/Engine/EditorBlueprintResources/StandardMacros.IncrementInt` (`self.Score`)
    (:`  `
      (`GameplayStatics.SpawnSoundAttached` "/Game/UI/Balloon_Pop_1.Balloon_Pop_1" (`self.DefaultSceneRoot`) "None" (0.0 0.0 0.0) (struct) "KeepRelativeOffset" false 1.0 1.0 0.0 null null))))

(event `self.ReceiveBeginPlay`
  (bind _returnvalue (`GameplayStatics.GetPlayerController` 0))
  (add `self.ScoreUpdater` (delegate `ScoreUpdater_AddScoreEvent`))
  (add `self.LevelBeginEvent` (delegate `StartLevelEvent`))
  (bind _returnvalue_2 (`|CreateWidget` "/Game/UI/BP_Health.BP_Health_C" _returnvalue))
  (`UserWidget.AddToViewport` _returnvalue_2 0)
  (bind _returnvalue_3 (`|CreateWidget` "/Game/UI/Score.Score_C" _returnvalue))
  (`UserWidget.AddToViewport` _returnvalue_3 0)
  (set `PlayerController.bShowMouseCursor` true _returnvalue)
  (set `PlayerController.bEnableClickEvents` true _returnvalue)
  (message `EnhancedInputSubsystemInterface.AddMappingContext` (pcsubsystem `EnhancedInputLocalPlayerSubsystem` _returnvalue) "/Game/Blueprints/Inputs/InputMappingContext.InputMappingContext" 0 (struct)))

(event `StartLevelEvent`
  (set `self.Score` 0)
  (set `self.LevelStarted` true)
  (`SceneComponent.SetVisibility` (`self.MergedChar`) true false)
  (`SceneComponent.K2_SetWorldLocation` (`self.MergedChar`) (`self.SpawnPosition`) false false)
  (set `self.CurrentSpeed` (`self.TargetSpeed`))
  (bind _returnvalue (`KismetSystemLibrary.K2_SetTimer` null "SpawnObstacle" 1.0 true))
  (set `self.SpawnerTimer` _returnvalue))

(event `self.ReceiveTick`
  (params (DeltaSeconds :type "Float (single-precision)"))
  (if (`self.LevelStarted`)
    (`SceneComponent.K2_AddLocalTransform` (`self.MergedChar`) (`KismetMathLibrary.MakeTransform` (`KismetMathLibrary.MakeVector` 0.0 (`self.CurrentSpeed`))) false false)))

(event `self.ReceiveAnyDamage`
  (params (Damage :type "Float (single-precision)") (DamageType :type "DamageType Object Reference") (InstigatedBy :type "Controller Object Reference") (DamageCauser :type "Actor Object Reference"))
  (if (not (`self.IsIntangible`))
    (bind _output_get (set `self.Health` (`KismetStringLibrary.Conv_StringToInt` (`KismetStringLibrary.Conv_DoubleToString` (- (`self.Health`) Damage)))))
    (if (<= _output_get 0)
      (`self.EndLevelEvent`)
      (`KismetSystemLibrary.K2_ClearAndInvalidateTimerHandle` (`self.SpawnerTimer`))
      (set `self.CurrentSpeed` 0.0)
      (`KismetSystemLibrary.K2_ClearAndInvalidateTimerHandle` (`self.SetFlashTimer`))
      (`SceneComponent.SetVisibility` (`self.MergedChar`) false false)
      (`self.Update High Score`)
      (else
        (cast `/Game/Blueprints/Obstacles/BP_WarningSign` DamageCauser
          (:`then`
            (`self.PlayPitfallAnimation` self))
          (:`CastFailed`
            _))
        (bind _returnvalue (`KismetSystemLibrary.K2_SetTimer` null "DamageFlash" 0.4 true))
        (set `self.SetFlashTimer` _returnvalue)
        ;[1 1 1] Without this logic sometimes after flashing the character remains  invisible
        (`KismetSystemLibrary.Delay` 4.0)
        (`KismetSystemLibrary.K2_ClearAndInvalidateTimerHandle` (`self.SetFlashTimer`))
        (`SceneComponent.SetVisibility` (`self.MergedChar`) true true)))))

(event `PlayPitfallAnimation`
  (params (`Player Object` :type "/Game/Blueprints/BP_Character Object Reference"))
  (bind _mergedchar (`/Game/Blueprints/BP_Character.MergedChar` `Player Object`))
  ;[1 1 1] Falling through the ground and respawning just slightly ahead of where it was.
  (set `self.PreviousPosition` (`SceneComponent.K2_GetComponentLocation` _mergedchar))
  (`PrimitiveComponent.SetSimulatePhysics` _mergedchar true)
  ;;[1 1 1] Without this then the hit event triggers multiple times on the same element
  (set `self.IsIntangible` true)
  (`KismetSystemLibrary.Delay` 1.0)
  (`PrimitiveComponent.SetSimulatePhysics` _mergedchar false)
  (`SceneComponent.K2_SetWorldLocation` (`self.MergedChar`) (+ (`self.PreviousPosition`) (100.0 0.0 0.0)) false false)
  (`KismetSystemLibrary.Delay` 1.0)
  (set `self.IsIntangible` false))

(fn `DamageFlash`
  (`SceneComponent.SetVisibility` (`self.MergedChar`) (not (`SceneComponent.bVisible` (`self.MergedChar`))) true))

(fn `SpawnObstacle`
  (locals (SpawnOffset :type "Transform Structure" :default "0.000000,100.000000,0.000000|0.000000,0.000000,0.000000|1.000000,1.000000,1.000000") (ArrowTransform :type "Transform Structure") (WarningSignOffset :type "Vector Structure" :default (0.0 -100.0 30.0)))
  (bind _returnvalue (`KismetMathLibrary.RandomIntegerInRange` 1 5))
  (set `local.ArrowTransform` (`SceneComponent.K2_GetComponentToWorld` (`self.Arrow`)))
  (if (== _returnvalue 1)
    (bind _returnvalue_2 (`|SpawnActorFromClass` "/Game/Blueprints/Obstacles/BP_Eagle.BP_Eagle_C" (`local.ArrowTransform`) "AlwaysSpawn" "MultiplyWithRoot" null null))
    (`SceneComponent.K2_AddRelativeLocation` (`/Game/Blueprints/Obstacles/BP_Eagle.low_poly_eagle` _returnvalue_2) (`KismetMathLibrary.MakeVector` 0.0 0.0 (`self.EagleHeight`)) false false)
    (elif (== _returnvalue 2)
      (`|SpawnActorFromClass` "/Game/Blueprints/Obstacles/Barrel.Barrel_C" (`local.ArrowTransform`) "Undefined" "MultiplyWithRoot" null null)
      (elif (== _returnvalue 3)
        (bind _returnvalue_3 (`|SpawnActorFromClass` "/Game/Blueprints/Obstacles/BP_WarningSign.BP_WarningSign_C" (`local.ArrowTransform`) "Undefined" "MultiplyWithRoot" null null))
        (`SceneComponent.K2_AddRelativeLocation` (`Actor.RootComponent` _returnvalue_3) (`local.WarningSignOffset`) false false)
        (elif (== _returnvalue 4)
          (bind _returnvalue_4 (`|SpawnActorFromClass` "/Game/Blueprints/Obstacles/BP_Rock.BP_Rock_C" (`local.ArrowTransform`) "Undefined" "MultiplyWithRoot" null null))
          (`SceneComponent.K2_AddRelativeLocation` (`/Game/Blueprints/Obstacles/BP_Rock.Rock8` _returnvalue_4) (`KismetMathLibrary.MakeVector` (`self.RockDistanceFromPlayer`) 0.0 (`self.RockHeight`)) false false)
          (else
            (`|SpawnActorFromClass` "/Game/Blueprints/Obstacles/BP_Trap.BP_Trap_C" (`local.ArrowTransform`) "Undefined" "MultiplyWithRoot" null null)))))))

(fn `Update High Score`
  (returns (Success :type Boolean))
  (locals (SaveSlotName :type String))
  (bind _returnvalue (`GameplayStatics.GetCurrentLevelName` true))
  (bind _returnvalue_2 (`KismetStringLibrary.Concat_StrStr` _returnvalue "HighScore"))
  (set `local.SaveSlotName` _returnvalue_2)
  (bind _returnvalue_3 (`GameplayStatics.DoesSaveGameExist` _returnvalue_2))
  (if _returnvalue_3
    (bind _returnvalue_4 (`GameplayStatics.LoadGameFromSlot` (`local.SaveSlotName`)))
    (bind _asbp_save_score (cast `/Game/Blueprints/BP_SaveScore` _returnvalue_4))
    (if (> (`self.Score`) (`/Game/Blueprints/BP_SaveScore.HighScore` _asbp_save_score))
      (bind _returnvalue_5 (`GameplayStatics.CreateSaveGameObject` "/Game/Blueprints/BP_SaveScore.BP_SaveScore_C"))
      (set `/Game/Blueprints/BP_SaveScore.HighScore` (`self.Score`) _returnvalue_5)
      (bind _returnvalue_6 (`GameplayStatics.SaveGameToSlot` _returnvalue_5 (`local.SaveSlotName`)))
      (return _returnvalue_6))
    (else
      (bind _returnvalue_7 (`GameplayStatics.CreateSaveGameObject` "/Game/Blueprints/BP_SaveScore.BP_SaveScore_C"))
      (set `/Game/Blueprints/BP_SaveScore.HighScore` (`self.Score`) _returnvalue_7)
      (bind _returnvalue_8 (`GameplayStatics.SaveGameToSlot` _returnvalue_7 (`local.SaveSlotName`)))
      (return _returnvalue_8))))

(fn `UserConstructionScript`)