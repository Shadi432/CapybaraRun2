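; BP_Eagle is a flying obstacle that homes in on BP_Character and can be clicked to destroy it and add score.
; On spawn it caches the player and plays a sound attached to them.
; Each tick it lerps the LowPolyEagle component from its current location toward the player's mesh with a growing alpha, so the approach is frame-rate dependent.
; Overlapping the player applies damage, plays a swipe sound and destroys the eagle.
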(event `self.ReceiveActorBeginOverlap`
  (params (OtherActor :type "Actor Object Reference"))
  (bind _asbp_character (cast `/Game/Blueprints/BP_Character` OtherActor))
  (`GameplayStatics.ApplyDamage` _asbp_character 1.0)
  (`GameplayStatics.SpawnSoundAttached` "/Game/SoundEffects/EagleSwipe.EagleSwipe" (`/Game/Blueprints/BP_Character.DefaultSceneRoot` _asbp_character) "None" (0.0 0.0 0.0) (struct) "KeepRelativeOffset" false 1.0 1.0 6.0 null null)
  (`self.K2_DestroyActor`))

(event `self.ReceiveTick`
  (params (DeltaSeconds :type "Float (single-precision)"))
  (`self.MoveTowardsPlayer`))

(event `self.ReceiveBeginPlay`
  (bind _returnvalue (`GameplayStatics.GetActorOfClass` "/Game/Blueprints/BP_Character.BP_Character_C"))
  (bind _output_get (set `self.Player` _returnvalue))
  (`GameplayStatics.SpawnSoundAttached` "/Game/SoundEffects/eagle-281163.eagle-281163" (`/Game/Blueprints/BP_Character.DefaultSceneRoot` _output_get) "None" (0.0 0.0 0.0) (struct) "KeepRelativeOffset" false 1.0 1.0 0.0 null null))

(event `self.ReceiveActorOnClicked`
  (params (ButtonPressed :type "Key Structure"))
  (`self.K2_DestroyActor`)
  (bind _returnvalue (`GameplayStatics.GetActorOfClass` "/Game/Blueprints/BP_Character.BP_Character_C"))
  (`/Game/Blueprints/BP_Character.ScoreUpdater_AddScoreEvent` _returnvalue))

(fn `MoveTowardsPlayer`
  (bind _returnvalue (+ (`self.LerpAlpha`) (`self.Speed`)))
  (if (>= _returnvalue 1.0)
    (set `self.LerpAlpha` 1.0)
    (else
      (bind _output_get (set `self.LerpAlpha` _returnvalue))))
  (`SceneComponent.K2_SetWorldLocation` (`self.low_poly_eagle`) (`KismetMathLibrary.VLerp` (`SceneComponent.K2_GetComponentLocation` (`self.low_poly_eagle`)) (`SceneComponent.K2_GetComponentLocation` (`/Game/Blueprints/BP_Character.MergedChar` (`self.Player`))) _output_get) false false))

(fn `UserConstructionScript`)