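; BP_Rock is a falling obstacle that damages the player on contact and awards score when clicked.
; Each Tick moves it down by Fallspeed and destroys it once the Rock8 component reaches world Z zero or below.
; Overlapping BP_Character applies damage, plays DeathEffect attached to the character and destroys the rock.
; Clicking destroys the rock and calls the character's add-score event.
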(event `self.ReceiveBeginPlay`
  (bind _returnvalue (`GameplayStatics.GetActorOfClass` "/Game/Blueprints/BP_Character.BP_Character_C"))
  (set `self.Player` _returnvalue))

(event `self.ReceiveActorBeginOverlap`
  (params (OtherActor :type "Actor Object Reference"))
  (bind _asbp_character (cast `/Game/Blueprints/BP_Character` OtherActor))
  (`GameplayStatics.ApplyDamage` _asbp_character 1.0)
  (`GameplayStatics.SpawnSoundAttached` "/Game/SoundEffects/DeathEffect.DeathEffect" (`/Game/Blueprints/BP_Character.DefaultSceneRoot` _asbp_character) "None" (0.0 0.0 0.0) (struct) "KeepRelativeOffset" false 1.0 1.0 12.0 null null)
  (`self.K2_DestroyActor`))

(event `self.ReceiveTick`
  (params (DeltaSeconds :type "Float (single-precision)"))
  (`self.K2_AddActorLocalOffset` (`KismetMathLibrary.MakeVector` 0.0 0.0 (* -1.0 (`self.Fallspeed`))))
  (if (<= (.z (`SceneComponent.K2_GetComponentLocation` (`self.Rock8`))) 0.0)
    (`self.K2_DestroyActor`)))

(event `self.ReceiveActorOnClicked`
  (params (ButtonPressed :type "Key Structure"))
  (`self.K2_DestroyActor`)
  (bind _returnvalue (`GameplayStatics.GetActorOfClass` "/Game/Blueprints/BP_Character.BP_Character_C"))
  (`/Game/Blueprints/BP_Character.ScoreUpdater_AddScoreEvent` _returnvalue))

(fn `UserConstructionScript`)